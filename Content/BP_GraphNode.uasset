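; BP_GraphNode is a graph node actor with a sphere and a sparkle component that highlights on pick input.
; The PickNode action and the left mouse button share one path that doubles the sphere's scale and shows the sparkles.
; The response comes from input events rather than the actor's empty click and release events, so it does not test which node is clicked.
; Nothing reverts the highlight.
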(event EventBeginPlay)

(event Collision|EventActorBeginOverlap
  (params (OtherActor :type Actor%20Object%20Reference)))

(event EventTick
  (params (DeltaSeconds :type Float%20%28single-precision%29)))

(event MouseInput|EventActorOnClicked
  (params (ButtonPressed :type Key%20Structure :default "None")))

(event EventActorOnReleased
  (params (ButtonReleased :type Key%20Structure :default "None")))

(event Input|ActionEvents|InputActionPickNode
  (params (Key :type Key%20Structure :default "None"))
  (:Pressed
    (Transformation|SetRelativeScale3D (Variables|Default|GetSphere) "2.000000,2.000000,2.000000")
    (Rendering|SetVisibility (Variables|Default|GetP_Sparkles) true false)))

(event Input|KeyboardEvents|NumPadZero
  (params (Key :type Key%20Structure :default "None")))

(event Input|MouseEvents|LeftMouseButton
  (params (Key :type Key%20Structure :default "None"))
  (:Pressed
    (Transformation|SetRelativeScale3D (Variables|Default|GetSphere) "2.000000,2.000000,2.000000")
    (Rendering|SetVisibility (Variables|Default|GetP_Sparkles) true false)))

(fn ConstructionScript)