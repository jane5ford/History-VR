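; BP_GraphNode is a graph node actor that BP_MotionController can pick up and release.
; Pickup attaches its root to the supplied component with world transform kept, shows the sparkle effect and clears the Rotable flag.
; Drop detaches it in place, hides the sparkles and sets Rotable again.
; Both events turn off sprite physics simulation, so a released node does not fall.
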(event EventBeginPlay)

(event EventPickup
  (params (AttachTo :type Scene%20Component%20Object%20Reference))
  (Physics|SetSimulatePhysics (Variables|Default|GetSpriteComponent) false)
  (Transformation|AttachComponentToComponent (VehicleSound|GetRootComponent) AttachTo "None" "KeepWorld" "KeepWorld" "KeepWorld" false)
  (Rendering|SetVisibility (Variables|Default|GetP_Sparkles) true false)
  (Variables|Default|SetRotable false))

(event EventDrop
  (Physics|SetSimulatePhysics (Variables|Default|GetSpriteComponent) false)
  (Transformation|DetachFromActor "KeepWorld" "KeepWorld" "KeepWorld")
  (Rendering|SetVisibility (Variables|Default|GetP_Sparkles) false false)
  (Variables|Default|SetRotable true))

(fn ConstructionScript)